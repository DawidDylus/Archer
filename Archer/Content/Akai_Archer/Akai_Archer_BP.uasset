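; Akai archer character Blueprint that handles the switch between the default and aiming camera views.
; Every Tick passes IsAiming to ChangeCamera, which eases the CameraBoom arm length, sideways socket offset and FollowCamera field of view toward aim or default targets.
; It lerps from each current value with a fixed alpha per frame, so the smoothing depends on frame rate.
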(event EventBeginPlay)

(event Collision|EventActorBeginOverlap
  (params (OtherActor :type Actor%20Object%20Reference)))

(event EventTick
  (params (DeltaSeconds :type Float%20%28single-precision%29))
  (CallFunction|ChangeCamera (Variables|Default|GetbIsAiming)))

(fn ConstructionScript)

(fn ChangeCamera
  (params (ChangeCamera :type Boolean))
  (bind _cameraboom (Variables|Default|GetCameraBoom))
  (bind _cameraboom_2 (Variables|Default|GetCameraBoom))
  (if ChangeCamera
    (Variables|/Script/Engine.SpringArmComponent|SetTargetArmLength _cameraboom_2 (Math|Float|Lerp (Variables|/Script/Engine.SpringArmComponent|GetTargetArmLength (Variables|Default|GetCameraBoom)) (Variables|Default|GetAimModeTargetArmLength) (Variables|Default|GetCameraMovementAlpha)))
    (Variables|/Script/Engine.SpringArmComponent|SetSocketOffset _cameraboom_2 (Math|Vector|MakeVector 0.0 (Math|Float|Lerp (.y (Variables|/Script/Engine.SpringArmComponent|GetSocketOffset (Variables|Default|GetCameraBoom))) (Variables|Default|GetAimModeCameraBoomSocketOffsetY) (Variables|Default|GetCameraMovementAlpha)) 0.0))
    (Variables|/Script/Engine.CameraComponent|SetFieldOfView (Variables|Default|GetFollowCamera) (Math|Float|Lerp (Variables|/Script/Engine.CameraComponent|GetFieldOfView (Variables|Default|GetFollowCamera)) (Variables|Default|GetAimModeFieldOfView) (Variables|Default|GetCameraMovementAlpha)))
    (else
      (Variables|/Script/Engine.SpringArmComponent|SetTargetArmLength _cameraboom (Math|Float|Lerp (Variables|/Script/Engine.SpringArmComponent|GetTargetArmLength (Variables|Default|GetCameraBoom)) (Variables|Default|GetDefaultTargetArmLength) (Variables|Default|GetCameraMovementAlpha)))
      (Variables|/Script/Engine.SpringArmComponent|SetSocketOffset _cameraboom (Math|Vector|MakeVector 0.0 (Math|Float|Lerp (.y (Variables|/Script/Engine.SpringArmComponent|GetSocketOffset (Variables|Default|GetCameraBoom))) (Variables|Default|GetDefaultCameraBoomSocketOffsetY) (Variables|Default|GetCameraMovementAlpha)) 0.0))
      (Variables|/Script/Engine.CameraComponent|SetFieldOfView (Variables|Default|GetFollowCamera) (Math|Float|Lerp (Variables|/Script/Engine.CameraComponent|GetFieldOfView (Variables|Default|GetFollowCamera)) (Variables|Default|GetDefaultFieldOfView) (Variables|Default|GetCameraMovementAlpha))))))